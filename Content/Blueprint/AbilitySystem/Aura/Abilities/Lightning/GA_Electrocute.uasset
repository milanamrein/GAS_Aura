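; Electrocute gameplay ability: a held lightning beam that roots the caster and chains from the target under the mouse to additional targets.
; A montage event starts the ShockLoop cues and a looping timer that commits mana cost and applies set-by-caller damage.
; Input release after a minimum spell time, empty mana or primary target death ends it.
; Debuffs are applied server-side only at the end, and cooldown is then committed.
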(event `self.K2_ActivateAbility`
  ;[1 1 1] Check if Actor implements CombatInterface
  (if (`KismetSystemLibrary.DoesImplementInterface` (`self.GetAvatarActorFromActorInfo`) "/Script/Aura.CombatInterface")
    ;[1 1 1] Setup Ability
    (bind (_asynctaskproxy _datahandle) (`TargetDataUnderMouse.CreateTargetDataUnderMouse`)
      (:`ValidData`
        (`self.StoreMouseDataInfo` (`AbilitySystemBlueprintLibrary.GetHitResultFromTargetData` _datahandle))
        (`self.StoreOwner`)
        (`|ExecutionSequence`
          (:`then_0`
            ;[1 1 1] Hide Mouse Cursor when Input is Held
            (set `PlayerController.bShowMouseCursor` false (`self.OwnerPlayerController`))
            (message `CombatInterface.UpdateFacingTarget` (`self.GetAvatarActorFromActorInfo`) (`self.MouseHitLocation`))
            (`self.K2_ExecuteGameplayCue` (struct :`TagName` "GameplayCue.ShockBurst"))
            (`AbilityTask_PlayMontageAndWait.CreatePlayMontageAndWaitProxy` "None" (`self.Montage_Electrocute`) 1.0 "None" false
              (:`then`
                (`AbilityTask_WaitGameplayEvent.WaitGameplayEvent` (struct :`TagName` "Event.Montage.Electrocute") null true
                  (:`EventReceived`
                    (`self.InShockLoop`)
                    ;[1 1 1] Activate Shock Loop Cue
                    (`self.SpawnElectricBeam`)
                    (bind _returnvalue (`KismetSystemLibrary.K2_SetTimerDelegate` (delegate `DamageAndCost`) (`self.DamageDeltaTime`) true))
                    (set `self.DamageAndCostTimer` _returnvalue))))))
          (:`then_1`
            (bind (_asynctaskproxy_2 _timeheld) (`AbilityTask_WaitInputRelease.WaitInputRelease` false)
              (:`OnRelease`
                (bind _output_get (set `self.Time Held` _timeheld))
                (if (< _output_get (`self.MinSpellTime`))
                  (`self.K2_HasAuthority`
                    (:`True`
                      ;[1 1 1] Make Spell last at least for the minimum amount of Spell Time
                      (`KismetSystemLibrary.Delay` (- (`self.MinSpellTime`) (`self.Time Held`)))
                      ;[1 1 1] End Ability only on Server
                      (`self.ClearTimerAndEndAbility` :!label _label))
                    (:`False`
                      ;[1 1 1] For Clients, only end Shock Loop
                      (`self.EndShockLoop`)))
                  (else
                    (goto _label)))))))))
    (else
      (`self.K2_EndAbility`))))

(event `DamageAndCost`
  ;[1 0 0] Apply Damage and Commit Cost
  (bind _returnvalue (`self.K2_CommitAbilityCost` false))
  ;;[1 1 1] Do we have enough Mana?
  (if _returnvalue
    (`self.ApplyDamage`)
    (else
      (`self.ClearTimerAndEndAbility`))))

(event `self.PrimaryTargetDied`
  (params (DeadActor :type "Actor Object Reference"))
  ;[1 0 0] Implement when First Target dies, end Ability
  (`GameplayCueFunctionLibrary.RemoveGameplayCueOnActor` DeadActor (struct :`TagName` "GameplayCue.ShockLoop") (`self.FirstTargetCueParams`))
  (`self.ClearTimerAndEndAbility`))

(event `self.AdditionalTargetDied`
  (params (DeadActor :type "Actor Object Reference"))
  ;[1 0 0] When Additional Target dies, remove from Additional Targets
  (`self.RemoveCueFromAdditionalTarget` DeadActor)
  (`KismetArrayLibrary.Array_RemoveItem` (`self.AdditionalTargets`) DeadActor))

(fn `AddCueToAdditionalTarget`
  (params (AdditionalTarget :type "Actor Object Reference"))
  (locals (TargetActor :type "Actor Object Reference"))
  (bind _targetactor (`local.TargetActor`))
  (bind _returnvalue (`AbilitySystemBlueprintLibrary.MakeGameplayCueParameters` 0.0 0.0 (struct) (struct) (struct) (struct) (struct) (`Actor.K2_GetActorLocation` _targetactor) (0.0 0.0 0.0) null null _targetactor null 1 1 (`Actor.RootComponent` (`self.MouseHitActor`))))
  (bind _output_get (set `local.TargetActor` AdditionalTarget))
  (`BlueprintMapLibrary.Map_Add` (`self.AdditionalActorsToCueParams`) _output_get _returnvalue)
  (`GameplayCueFunctionLibrary.AddGameplayCueOnActor` (`local.TargetActor`) (struct :`TagName` "GameplayCue.ShockLoop") _returnvalue))

(fn `ApplyDamage`
  (`self.ApplyDamageToSingleTarget` (`self.MouseHitActor`))
  (for _array_element (`self.AdditionalTargets`)
    (`self.ApplyDamageToSingleTarget` _array_element)))

(fn `ApplyDamageToSingleTarget`
  (params (Actor :type "Actor Object Reference"))
  (locals (ASC :type "AbilitySystemComponent Object Reference") (DamagedTarget :type "Actor Object Reference"))
  (bind _returnvalue (`AbilitySystemBlueprintLibrary.GetAbilitySystemComponent` (`local.DamagedTarget`)))
  (bind _output_get (set `local.DamagedTarget` Actor))
  (`/Engine/EditorBlueprintResources/StandardMacros.IsValid` _output_get
    (:`Is Valid`
      (bind _output_get_2 (set `local.ASC` (`self.GetAbilitySystemComponentFromActorInfo`)))
      (`/Engine/EditorBlueprintResources/StandardMacros.IsValid` _output_get_2
        (:`Is Valid`
          (`/Engine/EditorBlueprintResources/StandardMacros.IsValid` _returnvalue
            (:`Is Valid`
              ;[1 1 1] Only assign Damage as we don't want to apply Debuffs every time, only when ending the ShockLoop
              (bind _returnvalue_2 (`AbilitySystemBlueprintLibrary.AssignTagSetByCallerMagnitude` (`AbilitySystemComponent.MakeOutgoingSpec` (`local.ASC`) (`self.DamageEffectClass`) (`KismetMathLibrary.Conv_IntToDouble` (`self.GetAbilityLevel`)) (`AbilitySystemComponent.MakeEffectContext` (`local.ASC`))) (struct :`TagName` "Damage.Lightning") (`self.GetDamageAtLevel` (`BlueprintGameplayTagLibrary.MakeLiteralGameplayTag` (struct :`TagName` "Damage.Lightning")))))
              (`AbilitySystemComponent.BP_ApplyGameplayEffectSpecToSelf` _returnvalue _returnvalue_2))))))))

(fn `ClearTimerAndEndAbility`
  (`KismetSystemLibrary.K2_ClearAndInvalidateTimerHandle` (`self.DamageAndCostTimer`))
  (`self.EndShockLoop`)
  (`self.K2_CommitAbilityCooldown` false)
  (`self.ResetVariables`)
  (`self.K2_EndAbility`))

(fn `EndShockLoop`
  (bind _mousehitactor (`self.MouseHitActor`))
  (set `PlayerController.bShowMouseCursor` true (`self.OwnerPlayerController`))
  (message `CombatInterface.SetInShockLoop` (`self.GetAvatarActorFromActorInfo`) false)
  (`CharacterMovementComponent.SetMovementMode` (`Character.CharacterMovement` (`self.OwnerCharacter`)) "MOVE_Walking" 0)
  (if (`self.IsFirstTargetEnemy`)
    (message `CombatInterface.SetIsShocked` (`self.MouseHitActor`) false)
    (`GameplayCueFunctionLibrary.RemoveGameplayCueOnActor` _mousehitactor (struct :`TagName` "GameplayCue.ShockLoop") (`self.FirstTargetCueParams`))
    ;[1 1 1] Only apply Damage on Server
    (`self.K2_HasAuthority`
      (:`True`
        ;[1 1 1] Apply Debuff/Stun on Primary Target when Ability is ended
        (`AuraAbilitySystemLibrary.ApplyDamageEffect` (`self.MakeDamageEffectParamsFromClassDefaults` _mousehitactor)))
      (:`False`
        _))
    ;[1 1 1] Remove cue from Additional Targets too and apply Debuff/Stun on them on the Server
    (for _array_element (`self.AdditionalTargets`)
      (message `CombatInterface.SetIsShocked` (`self.MouseHitActor`) false)
      (`self.RemoveCueFromAdditionalTarget` _array_element)
      (`self.K2_HasAuthority`
        (:`True`
          (`AuraAbilitySystemLibrary.ApplyDamageEffect` (`self.MakeDamageEffectParamsFromClassDefaults` _array_element)))))
    (else
      (`GameplayCueFunctionLibrary.RemoveGameplayCueOnActor` (`self.GetAvatarActorFromActorInfo`) (struct :`TagName` "GameplayCue.ShockLoop") (`self.FirstTargetCueParams`)))))

(fn `InShockLoop`
  (message `CombatInterface.SetInShockLoop` (`self.GetAvatarActorFromActorInfo`) true)
  ;[1 1 1] Don't allow movement while casting Electrocute
  (`CharacterMovementComponent.DisableMovement` (`Character.CharacterMovement` (`self.OwnerCharacter`))))

(fn `RemoveCueFromAdditionalTarget`
  (params (AdditionalTarget :type "Actor Object Reference"))
  (bind (_value _returnvalue) (`BlueprintMapLibrary.Map_Find` (`self.AdditionalActorsToCueParams`) AdditionalTarget))
  (if _returnvalue
    (`GameplayCueFunctionLibrary.RemoveGameplayCueOnActor` AdditionalTarget (struct :`TagName` "GameplayCue.ShockLoop") _value)))

(fn `ResetVariables`
  (`KismetArrayLibrary.Array_Clear` (`self.AdditionalTargets`))
  (`BlueprintMapLibrary.Map_Clear` (`self.AdditionalActorsToCueParams`))
  (set `self.MouseHitActor` null)
  (set `self.IsFirstTargetEnemy` false)
  (set `self.Time Held` 0.0))

(fn `SpawnElectricBeam`
  (locals (SocketName :type Name :default "TipSocket"))
  ;[1 1 1] Get the first blocking Target of the TraceLine
  (`self.TraceFirstTarget` (`self.MouseHitLocation`) (`local.SocketName`))
  (bind _returnvalue (message `CombatInterface.GetWeapon` (`self.OwnerCharacter`)))
  (set `self.FirstTargetCueParams` (`AbilitySystemBlueprintLibrary.MakeGameplayCueParameters` 0.0 0.0 (struct) (struct) (struct) (struct) (struct) (`self.MouseHitLocation`) (0.0 0.0 0.0) null null (`self.MouseHitActor`) null 1 1 _returnvalue))
  (bind _output_get (set `self.IsFirstTargetEnemy` (`KismetSystemLibrary.DoesImplementInterface` (`self.MouseHitActor`) "/Script/Aura.CombatInterface")))
  ;[1 1 1] Is MouseHitActor an Enemy?
  (if _output_get
    ;[0 0.3855 1] Enemy
    (`GameplayCueFunctionLibrary.AddGameplayCueOnActor` (`self.MouseHitActor`) (struct :`TagName` "GameplayCue.ShockLoop") (`self.FirstTargetCueParams`))
    (message `CombatInterface.SetIsShocked` (`self.MouseHitActor`) true)
    (bind _outadditionaltargets (`self.StoreAdditionalTargets`))
    (bind _output_get_2 (set `self.AdditionalTargets` _outadditionaltargets))
    (for _array_element _output_get_2
      (`self.AddCueToAdditionalTarget` _array_element)
      (message `CombatInterface.SetIsShocked` _array_element true))
    (else
      ;[0 0.4722 1] Apply to Aura if MouseHitActor is a static object in the world
      (`GameplayCueFunctionLibrary.AddGameplayCueOnActor` (`self.GetAvatarActorFromActorInfo`) (struct :`TagName` "GameplayCue.ShockLoop") (`self.FirstTargetCueParams`)))))