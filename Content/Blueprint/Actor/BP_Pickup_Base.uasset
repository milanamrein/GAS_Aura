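; Base pickup actor that animates and sounds its spawn, idle motion and consumption.
; On BeginPlay a timeline drives height, scaled by a spawn apex, and uniform scale, with a one-shot impact sound when elevation dips below ground.
; When the timeline finishes, it starts sinusoidal movement and rotation.
; Tick applies the cached location and rotation, and destruction plays the consumed sound.
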(event `self.ReceiveBeginPlay`
  ;[1 1 1] Start Sin movement and Rotation effect
  (`GameplayStatics.PlaySoundAtLocation` (`self.SpawnSound`) (`self.K2_GetActorLocation`) (struct) 1.0 1.0 0.0 null null null null)
  (bind (_direction _elevation _scale) (`Timeline|PickupElevationTimeline`)
    (:`Update`
      (set `self.CalculatedLocation` (`self.CalculateElevation` _elevation))
      (`self.SetActorScale3D` (`KismetMathLibrary.MakeVector` _scale _scale _scale))
      (`self.PlayGroundHitSound` _elevation))
    (:`Finished`
      (`self.StartSinusoidalMovement`)
      (`self.StartRotation`))))

(event `self.ReceiveTick`
  (params (DeltaSeconds :type "Float (single-precision)"))
  ;[1 1 1] Move&Rotate Pickup
  (`self.K2_SetActorLocation` (`self.CalculatedLocation`))
  (`self.K2_SetActorRotation` (`self.CalculatedRotation`)))

(event `self.ReceiveDestroyed`
  ;[1 1 1] Consume Pickup
  (`GameplayStatics.PlaySoundAtLocation` (`self.ConsumedSound`) (`self.K2_GetActorLocation`) (struct) 1.0 1.0 0.0 null null null null))

(fn `CalculateElevation`
  (params (Elevation :type "Float (double-precision)"))
  (returns (ReturnValue :type "Vector Structure"))
  (bind (_initiallocation_x _initiallocation_y _initiallocation_z) (`KismetMathLibrary.BreakVector` (`self.InitialLocation`)))
  (return (`KismetMathLibrary.MakeVector` _initiallocation_x _initiallocation_y (+ (* Elevation (`self.SpawnApex`)) _initiallocation_z))))

(fn `PlayGroundHitSound`
  (params (Elevation :type "Float (double-precision)"))
  (if (< Elevation -0.1)
    (`/Engine/EditorBlueprintResources/StandardMacros.DoOnce` false
      (:`Completed`
        (`GameplayStatics.PlaySoundAtLocation` (`self.GroundImpactSound`) (`self.K2_GetActorLocation`) (struct) 1.0 1.0 0.0 null null null null)))))

(fn `UserConstructionScript`)