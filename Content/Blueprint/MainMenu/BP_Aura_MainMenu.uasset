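; BP_Aura_MainMenu is the animated Aura display actor for the main menu, which also opens the menu UI.
; On BeginPlay it stores the fireball's location, adds WBP_MainMenu to the viewport, sets UI-only input and shows the cursor.
; Each tick, a sine of wrapped accumulated time bobs the fireball in her hand vertically while the magic circle decal rotates at a configurable rate.
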(event `self.ReceiveBeginPlay`
  (set `self.FireBallInitialLocation` (`SceneComponent.K2_GetComponentLocation` (`self.FireBall`)))
  (`self.AddMainMenuToViewport`))

(event `self.ReceiveTick`
  (params (DeltaSeconds :type "Float (single-precision)"))
  ;[1 0 0] Make FireBall in Aura's hand float up and down
  (`self.UpdateTime` DeltaSeconds)
  (`SceneComponent.K2_SetWorldLocation` (`self.FireBall`) (+ (`self.FireBallInitialLocation`) (`KismetMathLibrary.MakeVector` 0.0 0.0 (`self.SinTime`))) false false)
  (`self.RotateMagicCircle` DeltaSeconds))

(fn `AddMainMenuToViewport`
  (bind _returnvalue (`GameplayStatics.GetPlayerController` 0))
  (bind _returnvalue_2 (`|CreateWidget` "/Game/Blueprint/UI/MainMenu/WBP_MainMenu.WBP_MainMenu_C"))
  (`UserWidget.AddToViewport` _returnvalue_2 0)
  (`WidgetBlueprintLibrary.SetInputMode_UIOnlyEx` _returnvalue _returnvalue_2)
  (set `PlayerController.bShowMouseCursor` true _returnvalue))

(fn `RotateMagicCircle`
  (params (DeltaTime :type "Float (double-precision)"))
  (`SceneComponent.K2_AddLocalRotation` (`self.Decal`) (`KismetMathLibrary.MakeRotator` (* DeltaTime (`self.MagicCircleRotationRate`))) false false))

(fn `SinTime`
  (returns (ReturnValue :type "Float (double-precision)"))
  (return (* (`KismetMathLibrary.Sin` (`self.Time`)) (`self.Amplitude`))))

(fn `UpdateTime`
  (params (DeltaTime :type "Float (double-precision)"))
  (bind _output_get (set `self.Time` (+ DeltaTime (`self.Time`))))
  ;[1 1 1] 2 pi (3.14x2) is the period for sin()
  (if (> _output_get 6.28318)
    (set `self.Time` 0.0)))

(fn `UserConstructionScript`)